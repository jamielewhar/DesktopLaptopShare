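; Wooden sword weapon Blueprint that deals melee damage to opposing-team Entities through a toggleable HitBox.
; On overlap, it gets damage from the possessing Entity's CalculateDamage and applies it as negative health to overlapping Entities on other teams.
; EnemiesHit prevents repeat hits until cleared; EnableHitbox and DisableHitbox switch query collision.
; ClearEnemiesHit removes elements while iterating the same array, so it can skip entries.
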(event `self.ReceiveTick`
  (params (DeltaSeconds :type "Float (single-precision)")))

(event `self.ReceiveActorBeginOverlap`
  (params (OtherActor :type "Actor Object Reference"))
  ;[1 1 1] Calculate Damage Using Player Stats
  (bind _asentity (cast `/Game/Blueprints/Characters/Entity` (`self.PossessingEntity`)))
  (bind _sending_damage (`/Game/Blueprints/Characters/Entity.CalculateDamage` _asentity))
  (set `self.Damage` (* _sending_damage -1.0))
  ;[1 1 1] Determine Enemies/Allies
  (set `self.Team` (`/Game/Blueprints/Characters/Entity.Team` _asentity))
  ;[1 1 1] Continue BP for Every Overlapping Character
  (for _array_element (`self.GetOverlappingActors` "/Game/Blueprints/Characters/Entity.Entity_C")
    ;[1 1 1] Check if they are on team
    (bind _asentity_2 (cast `/Game/Blueprints/Characters/Entity` _array_element))
    (if (not (== (`self.Team`) (`/Game/Blueprints/Characters/Entity.Team` _asentity_2)))
      ;[1 1 1] Have I Already Hit This Enemy?
      (if (not (`KismetArrayLibrary.Array_Contains` (`self.EnemiesHit`) _asentity_2))
        ;[1 1 1] Damage Enemies
        (`/Game/Blueprints/Characters/Entity.AdjustHealth` _asentity_2 (`self.Damage`))
        ;[1 1 1] Add to Enemies Hit (testing for attack delay
        (`KismetArrayLibrary.Array_Add` (`self.EnemiesHit`) _asentity_2)))))

(fn `Clear Enemies Hit`
  (bind _enemieshit (`self.EnemiesHit`))
  (bind _returnvalue (`KismetArrayLibrary.Array_Length` _enemieshit))
  (if (> _returnvalue 0)
    (for _array_element _enemieshit
      (`KismetArrayLibrary.Array_RemoveItem` _enemieshit _array_element)
      (`KismetSystemLibrary.PrintString` (`KismetStringLibrary.Conv_IntToString` _returnvalue)))))

(fn `Disable Hitbox`
  (`PrimitiveComponent.SetCollisionEnabled` (`self.HitBox`) "NoCollision"))

(fn `EnableHitbox`
  (`PrimitiveComponent.SetCollisionEnabled` (`self.HitBox`) "QueryOnly"))

(fn `UserConstructionScript`)