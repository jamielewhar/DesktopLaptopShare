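; Base interactable actor that registers itself with the player character when the player overlaps it.
; On begin overlap it passes itself to the Player's UpdateInteractable.
; On end overlap it clears the Player's InteractObject if that still points to itself.
; Interact is an empty function taking the interacting object, with no behavior defined here.
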(event `self.ReceiveActorEndOverlap`
  (params (OtherActor :type "Actor Object Reference"))
  (bind _returnvalue (`GameplayStatics.GetPlayerCharacter` 0))
  (if (== OtherActor _returnvalue)
    (bind _asplayer (cast `/Game/Blueprints/Characters/Player` _returnvalue))
    (if (== (`/Game/Blueprints/Characters/Player.InteractObject` _asplayer) self)
      (set `/Game/Blueprints/Characters/Player.InteractObject` null _asplayer))))

(event `self.ReceiveActorBeginOverlap`
  (params (OtherActor :type "Actor Object Reference"))
  (bind _returnvalue (`GameplayStatics.GetPlayerCharacter` 0))
  (if (== OtherActor _returnvalue)
    (bind _asplayer (cast `/Game/Blueprints/Characters/Player` _returnvalue))
    (`/Game/Blueprints/Characters/Player.UpdateInteractable` _asplayer self)))

(fn `Interact`
  (params (ObjectThatInteracted :type "Actor Object Reference")))

(fn `UserConstructionScript`)