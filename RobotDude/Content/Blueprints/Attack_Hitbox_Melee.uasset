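; Short-lived melee attack hitbox actor that damages Entities on a different team from its instigator.
; On overlap, it gets damage from the instigator's CalculateDamage, negates it and passes it to AdjustHealth on each overlapping opposing Entity.
; It destroys itself when it hits, or otherwise after a half-second Delay driven from Tick.
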(event `self.ReceiveBeginPlay`)

(event `self.ReceiveActorBeginOverlap`
  (params (OtherActor :type "Actor Object Reference"))
  (bind _asentity (cast `/Game/Blueprints/Characters/Entity` (`self.GetInstigator`)))
  (bind _sending_damage (`/Game/Blueprints/Characters/Entity.CalculateDamage` _asentity))
  (set `self.Damage` (* _sending_damage -1.0))
  (set `self.Team` (`/Game/Blueprints/Characters/Entity.Team` _asentity))
  (for _array_element (`self.GetOverlappingActors` "/Game/Blueprints/Characters/Entity.Entity_C")
    (bind _asentity_2 (cast `/Game/Blueprints/Characters/Entity` _array_element))
    (if (not (== (`self.Team`) (`/Game/Blueprints/Characters/Entity.Team` _asentity_2)))
      (`/Game/Blueprints/Characters/Entity.AdjustHealth` _asentity_2 (`self.Damage`))
      (`self.K2_DestroyActor`))))

(event `self.ReceiveTick`
  (params (DeltaSeconds :type "Float (single-precision)"))
  (`KismetSystemLibrary.Delay` 0.5)
  (`self.K2_DestroyActor`))

(fn `UserConstructionScript`)