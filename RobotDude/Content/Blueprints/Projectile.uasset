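; Projectile actor that damages entities on an opposing team.
; On begin overlap, it casts both its instigator and the overlapped actor to Entity and compares their Team values.
; If the teams differ, it passes Damage to the target's AdjustHealth and destroys itself; same-team and non-Entity overlaps are ignored.
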(event `self.ReceiveActorBeginOverlap`
  (params (OtherActor :type "Actor Object Reference"))
  ;[1 1 1] This Projectile = Instigators Team
  (bind _asentity (cast `/Game/Blueprints/Characters/Entity` (`self.GetInstigator`)))
  (set `self.Team` (`/Game/Blueprints/Characters/Entity.Team` _asentity))
  (bind _asentity_2 (cast `/Game/Blueprints/Characters/Entity` OtherActor))
  (if (not (== (`self.Team`) (`/Game/Blueprints/Characters/Entity.Team` _asentity_2)))
    (`/Game/Blueprints/Characters/Entity.AdjustHealth` _asentity_2 (`self.Damage`))
    (`self.K2_DestroyActor`)))

(fn `UserConstructionScript`)