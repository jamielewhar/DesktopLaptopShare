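; Enemy character that attacks and jumps on a timer and drops experience when it dies.
; It extends a parent character, driving inherited Attack by simulating a button press from Delay nodes on Tick, alongside a timed Jump.
; A health-adjust event feeds the health ratio to its HP bar widget.
; Death waits briefly, spawns an ExpPickup carrying its ExpValue at the FirePoint bone, then destroys the actor.
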(event `self.AdjustHealthPercent`
  (bind _current_health (`self.Current Health`))
  (bind _output_get (set `self.HealthPercent` (/ _current_health (`self.Max Health`))))
  (set `/Game/Blueprints/UI/HPBar.healthPercent` _output_get (`self.myHPBar`))
  (set `self.Previous Health` _current_health))

(event `self.ReceiveBeginPlay`
  (`parent.ReceiveBeginPlay`)
  (set `self.ExpValue` 10.0)
  (set `self.FirePoint` "FirePoint")
  (bind _ashpbar (cast `/Game/Blueprints/UI/HPBar` (`WidgetComponent.GetUserWidgetObject` (`self.HPBar`))))
  (set `self.myHPBar` _ashpbar)
  (set `self.MyDamageColor` (struct :`R` 1.0 :`G` 1.0 :`B` 1.0 :`A` 1.0)))

(event `self.ReceiveTick`
  (params (DeltaSeconds :type "Float (single-precision)"))
  (if (`self.Attack Button Down`)
    (`self.Attack`)
    (set `self.Attack Button Down` false))
  (`parent.ReceiveTick` 0.0)
  (`|ExecutionSequence`
    (:`then_0`
      (`KismetSystemLibrary.Delay` 2.0)
      (set `self.Attack Button Down` true))
    (:`then_1`
      (`KismetSystemLibrary.Delay` 2.0)
      (`self.Jump`)
      (set `self.Jumping` true))))

(event `self.Death`
  (bind _outposition (`SkinnedMeshComponent.TransformFromBoneSpace` :`self` (`self.Mesh`) :`BoneName` "FirePoint"))
  (`KismetSystemLibrary.Delay` 0.5)
  (bind _returnvalue (`|SpawnActorFromClass` "/Game/Blueprints/ExpPickup.ExpPickup_C" (`KismetMathLibrary.MakeTransform` _outposition) "Undefined" "OverrideRootScale" null self))
  (set `/Game/Blueprints/PickUp.Value` (`self.ExpValue`) _returnvalue)
  (`self.K2_DestroyActor`))

(fn `UserConstructionScript`
  (`parent.UserConstructionScript`))