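; HealingItem is an item actor named "Healing" that adjusts the player's health when interacted with.
; On Interact it casts the interacting object to Player, passes Value to AdjustHealth, then destroys itself; other objects have no effect.
; BeginPlay sets the name, while overlap and construction only call the parent implementations and Tick is disabled.
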(event `self.ReceiveBeginPlay`
  (`parent.ReceiveBeginPlay`)
  (set `self.Name` "Healing"))

(event `self.ReceiveActorBeginOverlap`
  (params (OtherActor :type "Actor Object Reference"))
  (`parent.ReceiveActorBeginOverlap` OtherActor))

(event `self.Interact`
  (params (ObjectThatInteracted :type "Actor Object Reference"))
  (bind _asplayer (cast `/Game/Blueprints/Characters/Player` ObjectThatInteracted))
  (`/Game/Blueprints/Characters/Entity.AdjustHealth` _asplayer (`self.Value`))
  (`self.K2_DestroyActor`))

(fn `UserConstructionScript`
  (`parent.UserConstructionScript`))