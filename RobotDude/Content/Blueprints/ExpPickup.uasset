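; Experience pickup actor that grants experience to the player when used.
; On begin play it takes its value from the ExpValue of its Entity instigator.
; Its Use event adds that value to player 0's character through AddExp, prints a debug string and destroys the pickup.
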(event `self.ReceiveBeginPlay`
  (`parent.ReceiveBeginPlay`)
  (bind _asentity (cast `/Game/Blueprints/Characters/Entity` (`self.Instigator`)))
  (set `self.Value` (`/Game/Blueprints/Characters/Entity.ExpValue` _asentity)))

(event `self.Use`
  (bind _asplayer (cast `/Game/Blueprints/Characters/Player` (`GameplayStatics.GetPlayerCharacter` 0)))
  (`KismetSystemLibrary.PrintString` "Hello")
  (`/Game/Blueprints/Characters/Player.AddExp` _asplayer (`self.Value`))
  (`self.K2_DestroyActor`))

(fn `UserConstructionScript`
  (`parent.UserConstructionScript`))